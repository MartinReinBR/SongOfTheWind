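; BP_FG_GlidingPlayerState is the player's gliding state, which drives the glide noise on BP_FG_PlayerCharacter.
; It caches the owning character on BeginPlay, toggles the noise on state entry and stops it on exit.
; Each tick it passes the character's speed, taken as velocity length, to update that noise.
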(event EventBeginPlay
  (bind _asbp_fg_player_character (Utilities|Casting|CastToBP_FG_PlayerCharacter (Components|GetOwner)))
  (Variables|Default|SetPlayerRef _asbp_fg_player_character))

(event EventOnStateEnter
  (Default|ToggleGlideNoise (Variables|Default|GetPlayerRef)))

(event EventOnStateExit
  (Default|StopGlideNoise (Variables|Default|GetPlayerRef)))

(event EventTick
  (params (DeltaSeconds :type Float%20%28single-precision%29))
  (Default|UpdateGlideNoise (Variables|Default|GetPlayerRef) (Math|Vector|VectorLength (Transformation|GetVelocity (Variables|Default|GetPlayerRef)))))