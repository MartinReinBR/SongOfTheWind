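; Player locomotion state Blueprint that spawns a landing dust effect when the player character lands.
; On the land event it compares vertical velocity to a hard-landing threshold, choosing the regular puff at actor scale for hard landings or a small puff otherwise.
; Both Niagara systems spawn just below the actor location with auto-release pooling, and the landing velocity is also printed to screen.
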(event EventBeginPlay)

(event EventTick
  (params (DeltaSeconds :type Float%20%28single-precision%29)))

(event EventOnPlayerLand
  (params (PlayerCharacter :type FG%20Player%20Character%20Object%20Reference))
  (bind _returnvalue (Transformation|GetActorLocation PlayerCharacter))
  (bind _returnvalue_2 (Transformation|GetVelocity PlayerCharacter))
  (bind _returnvalue_3 (Transformation|GetActorRotation PlayerCharacter))
  (bind _returnvalue_4 (- (.z _returnvalue) 1e+02))
  (Development|PrintString (Utilities|String|ToString(Float) (.z _returnvalue_2)))
  (if (>= (Variables|Default|GetHardlandTreshold) (.z _returnvalue_2))
    (Niagara|SpawnSystematLocation "/Game/Art/ParticleEffects/NM_LandingPuff.NM_LandingPuff" (Math|Vector|MakeVector (.x _returnvalue) (.y _returnvalue) _returnvalue_4) _returnvalue_3 (Transformation|GetActorScale3D PlayerCharacter) true true "AutoRelease")
    (else
      (Niagara|SpawnSystematLocation "/Game/Art/ParticleEffects/NM_LandingPuffSmall.NM_LandingPuffSmall" (Math|Vector|MakeVector (.x _returnvalue) (.y _returnvalue) _returnvalue_4) _returnvalue_3 "1.000000,1.000000,1.000000" true true "AutoRelease"))))