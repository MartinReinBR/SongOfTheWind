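; Idle sub-state of the player's locomotion states, currently with no active behavior of its own.
; BeginPlay calls the parent, then casts and caches the owning player character.
; State enter is empty and Tick is disabled; disconnected nodes hold a parent enter call, a debug print and a pooled Niagara landing-puff spawn at the player's location.
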(event EventBeginPlay
  (|CallParentFunction)
  (bind _asbp_fg_player_character (Utilities|Casting|CastToBP_FG_PlayerCharacter (Class|FGPlayerState|GetFGPlayer)))
  (Variables|Default|SetAs%20BP%20FG%20Player%20Character _asbp_fg_player_character))

(event EventTick
  (params (DeltaSeconds :type Float%20%28single-precision%29)))

(event EventOnStateEnter)