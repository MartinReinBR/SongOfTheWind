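; Player character Blueprint with gliding, interaction, a pause menu and a debug HUD toggle.
; Tick drives the glider trail Niagara parameters from collider velocity, active only while the state machine's top state is gliding.
; Collider overlaps track an Int_interact actor that F messages, while menu open and close events shift the camera's truck offset.
; Helper functions manage a speed-scaled glide whoosh sound.
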(event Custom|OnMenuOpen
  (Class|FGCamera|SetTruckOffset (Variables|Default|GetMyCamera) -225.0))

(event Custom|OnMenuClose
  (Class|FGCamera|SetTruckOffset (Variables|Default|GetMyCamera) 0.0))

(event EventBeginPlay
  (bind _returnvalue (UserInterface|CreateWidget "/Game/Blueprints/Menu/Settings/Pause_Menu.Pause_Menu_C" (Game|GetPlayerController 0)))
  (bind _output_get (Variables|FGPlayerCharacter|SetMainMenuWidget _returnvalue))
  (EventDispatchers|BindEventtoOnOpen _output_get (delegate Custom|OnMenuOpen))
  (EventDispatchers|BindEventtoOnClose _output_get (delegate Custom|OnMenuClose)))

(event EventDeathcall
  (Default|CallDeath))

(event EventTick
  (params (DeltaSeconds :type Float%20%28single-precision%29))
  (bind _glidertrail (Variables|Default|GetGliderTrail))
  (bind _statemachine (Variables|Default|GetStateMachine))
  (bind _glidingcorestate (Variables|Default|GetGlidingCoreState))
  (bind _returnvalue (Class|FGSFSM|TopIsEqual _statemachine _glidingcorestate))
  (bind _returnvalue_2 (Math|Conversions|ToFloat(Boolean) _returnvalue))
  (bind _returnvalue_3 (Physics|GetPhysicsLinearVelocity (Variables|Default|GetCollider) "None"))
  (Niagara|SetNiagaraVariable(Float) _glidertrail "TrailSpeed" (* (/ (Math|Vector|VectorLength _returnvalue_3) 1.5e+02) _returnvalue_2))
  (Niagara|SetNiagaraVariable(Float) _glidertrail "FlightTrail" (* 1e+02 _returnvalue_2)))

(event Input|KeyboardEvents|1
  (params (Key :type Key%20Structure))
  (bind _returnvalue (Game|GetPlayerController 0))
  (:Pressed
    (Utilities|FlowControl|FlipFlop
      (:A
        (Variables|/Script/Engine.PlayerController|SetbShowMouseCursor _returnvalue true)
        (bind _returnvalue_2 (UserInterface|CreateWidget "/Game/Maps/Test/SushantTestLevel/Blueprints/HUD_DebugValues.HUD_DebugValues_C"))
        (UserInterface|Viewport|AddtoViewport _returnvalue_2 0))
      (:B
        (Variables|/Script/Engine.PlayerController|SetbShowMouseCursor _returnvalue false)
        (Widget|RemovefromParent _returnvalue_2)))))

(event Input|KeyboardEvents|4
  (params (Key :type Key%20Structure))
  (:Pressed
    (Default|TryOpenElseClose (Variables|FGPlayerCharacter|GetMainMenuWidget))))

(fn ConstructionScript)

(fn ToggleGlideNoise
  (bind _returnvalue (AddComponent|AddAudioComponent false))
  (Variables|Default|SetGliderWooshSound _returnvalue))

(fn StopGlideNoise
  (Audio|Components|Audio|Stop (Variables|Default|GetGliderWooshSound)))

(fn UpdateGlideNoise
  (params (VelocityDist :type Float%20%28single-precision%29))
  (bind _gliderwooshsound (Variables|Default|GetGliderWooshSound))
  (Utilities|IsValid _gliderwooshsound
    (:Is%20Valid
      (if true
        (Audio|Components|Audio|SetPitchMultiplier _gliderwooshsound (Math|Float|Clamp(Float) (/ VelocityDist 1e+03) 1.0 2.0))
        (Audio|Components|Audio|SetVolumeMultiplier _gliderwooshsound (Math|Float|Clamp(Float) (/ VelocityDist 2e+03)) :!class /Script/Engine.AudioComponent)))))

(event OnComponentBeginOverlap(Collider)
  (params (OverlappedComponent :type Primitive%20Component%20Object%20Reference) (OtherActor :type Actor%20Object%20Reference) (OtherComp :type Primitive%20Component%20Object%20Reference) (OtherBodyIndex :type Integer) (bFromSweep :type Boolean) (SweepResult :type Hit%20Result%20Structure%20%28by%20ref%29))
  (if (Utilities|DoesObjectImplementInterface OtherActor "/Game/Maps/Test/SushantTestLevel/Interfaces/int_interact.int_interact_C")
    (Variables|Default|SetInteractActor OtherActor)))

(event OnComponentEndOverlap(Collider)
  (params (OverlappedComponent :type Primitive%20Component%20Object%20Reference) (OtherActor :type Actor%20Object%20Reference) (OtherComp :type Primitive%20Component%20Object%20Reference) (OtherBodyIndex :type Integer))
  (if (== OtherActor (Variables|Default|GetInteractActor))
    (Variables|Default|SetInteractActor 0)))

(event Input|KeyboardEvents|F
  (params (Key :type Key%20Structure))
  (:Pressed
    (Class|IntInteract|InteractButton(Message) (Variables|Default|GetinteractActor))))