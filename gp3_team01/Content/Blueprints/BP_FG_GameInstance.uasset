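; Game instance Blueprint that applies startup display settings and exposes the player camera's orientation.
; On init it caps the frame rate, enables VSync, applies the user settings and resets LotusScore.
; GetCameraOrientation calls its parent, then returns the rotation of the first player's camera manager.
; GetMainCamera is an empty stub, with its camera manager lookup left unconnected.
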(event EventInit
  (bind _returnvalue (Settings|GetGameUserSettings))
  (Class|GameUserSettings|SetFrameRateLimit _returnvalue 6e+01)
  (Class|GameUserSettings|SetVSyncEnabled _returnvalue true)
  (Class|GameUserSettings|ApplySettings _returnvalue true)
  (Class|DAFGIntegerData|Reset (Variables|Default|GetLotusScore)))

(fn GetMainCamera
  (return 0))

(fn GetCameraOrientation
  (|CallParentFunction)
  (return (Camera|GetCameraRotation (Game|GetPlayerCameraManager 0))))