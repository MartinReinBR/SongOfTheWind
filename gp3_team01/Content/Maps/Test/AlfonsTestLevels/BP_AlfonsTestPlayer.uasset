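; Test player Blueprint in Alfons's test maps that moves from two-axis input.
; Each Tick normalizes the Vertical and Horizontal axes into a flat vector and passes it to FGLocomotion.Move with Acceleration and MaxSpeed.
; The gravity step adds an acceleration force to the Capsule, but its vector is zero, so it has no effect.
; BeginPlay sets SetFramerate to zero.
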(event EventBeginPlay
  (Variables|Default|SetSetFramerate 0.0))

(event Collision|EventActorBeginOverlap
  (params (OtherActor :type Actor%20Object%20Reference)))

(event EventTick
  (params (DeltaSeconds :type Float%20%28single-precision%29))
  ;[1 1 1] Gravity
  (Physics|AddForce (Variables|Default|GetCapsule) "0, 0, 0" "None" true)
  ;[1 1 1] Apply movement
  (Class|FGLocomotionComponent|Move (Variables|Default|GetFG_Locomotion) (Math|Conversions|ToVector(Vector2D) (Math|Vector2D|Normalize2D (Math|Vector2D|MakeVector2D (Input|AxisValues|GetVertical) (Input|AxisValues|GetHorizontal)))) (Variables|Default|GetAcceleration) (Variables|Default|GetMaxSpeed)))

(fn ConstructionScript)