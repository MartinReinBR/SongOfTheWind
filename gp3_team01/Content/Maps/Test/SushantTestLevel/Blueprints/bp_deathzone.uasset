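; Death zone trigger in a test level that sends the player back to a spawn transform.
; On BeginPlay it finds the BP_FG_PlayerCharacter, calls its DeathcallMessage and binds DeathCall to its death event.
; The player pawn overlapping the Box also calls DeathCall, which starts a camera fade from black with audio, teleports the player to SpawnTransform and prints a debug string.
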(event OnComponentBeginOverlap(Box)
  (params (OverlappedComponent :type Primitive%20Component%20Object%20Reference) (OtherActor :type Actor%20Object%20Reference) (OtherComp :type Primitive%20Component%20Object%20Reference) (OtherBodyIndex :type Integer) (bFromSweep :type Boolean) (SweepResult :type Hit%20Result%20Structure%20%28by%20ref%29))
  (if (== OtherActor (Game|Player|GetPlayerPawn 0))
    (CallFunction|DeathCall)))

(event Custom|DeathCall
  (bind _spawntransform (Variables|Default|GetSpawnTransform))
  (CameraFades|StartCameraFade (Game|GetPlayerCameraManager 0) 2.0 0.0 2.0 "(R=0.000000,G=0.000000,B=0.000000,A=1.000000)" true true)
  (Transformation|Teleport (Variables|Default|GetPlayerRef) (.location _spawntransform) (.rotation _spawntransform))
  (Development|PrintString "Hello"))

(event EventBeginPlay
  (bind _returnvalue (Actor|GetActorOfClass "/Game/Blueprints/Player/BP_FG_PlayerCharacter.BP_FG_PlayerCharacter_C"))
  (bind _output_get (Variables|Default|SetPlayerRef _returnvalue))
  (Class|IntDeath|Deathcall(Message) _output_get)
  (EventDispatchers|BindEventtoDeath (Variables|Default|GetPlayerRef) (delegate Custom|DeathCall)))

(fn ConstructionScript)