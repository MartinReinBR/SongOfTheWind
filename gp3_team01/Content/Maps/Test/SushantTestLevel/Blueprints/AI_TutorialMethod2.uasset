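; Tutorial guide AI that travels along a level spline and shows timed text prompts at trigger boxes.
; On BeginPlay it finds BP_TutorialPath and, if the player's world X passes a one-time threshold check, starts a timeline moving it along the spline over TimeToComplete.
; Its sphere overlapping any of the first three TriggerBoxes, matched by array index, sets TutorialText and briefly shows HUD_Tutorial.
; Impulse and homing-target logic is unconnected.
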(event EventBeginPlay
  (Utilities|FlowControl|Sequence
    (:then_0
      (bind _returnvalue (Actor|GetActorOfClass "/Game/Maps/Test/SushantTestLevel/Blueprints/BP_TutorialPath.BP_TutorialPath_C"))
      (Variables|Default|SetSplineREF _returnvalue)
      (if (<= (.x (Transformation|GetActorLocation (Game|Player|GetPlayerPawn 0))) (Variables|Default|GetDistancebetweenPlayer))
        (CallFunction|MoveAIto)))
    (:then_1
      (bind _outactors (Actor|GetAllActorsOfClass "/Script/Engine.TriggerBox"))
      (Variables|Default|SetBoxTriggers _outactors))))

(event Custom|MoveAITo
  (bind _splineref (Variables|Default|GetSplineREF))
  (bind _spline (Variables|/Game/Maps/Test/SushantTestLevel/Blueprints/BP_TutorialPath.BP_TutorialPath_C|GetSpline _splineref))
  (Components|Timeline|SetPlayRate (Variables|Default|GetMoveAITimeline) (/ 1.0 (Variables|Default|GetTimeToComplete)))
  (bind _movetrack (Timeline|MoveAITimeline Play)
    (:Update
      (Transformation|SetActorTransform (Math|Transform|MakeTransform (Spline|GetLocationatDistanceAlongSpline _spline (Math|Float|Lerp 0.0 (Spline|GetSplineLength (Variables|/Game/Maps/Test/SushantTestLevel/Blueprints/BP_TutorialPath.BP_TutorialPath_C|GetSpline (Variables|Default|GetSplineREF))) _movetrack) "World") (Spline|GetRotationatDistanceAlongSpline _spline (Math|Float|Lerp 0.0 (Spline|GetSplineLength (Variables|/Game/Maps/Test/SushantTestLevel/Blueprints/BP_TutorialPath.BP_TutorialPath_C|GetSpline (Variables|Default|GetSplineREF))) _movetrack) "Local") "1,1,1")))))

(fn ConstructionScript)

(fn HudON
  (bind _returnvalue (UserInterface|CreateWidget "/Game/Maps/Test/SushantTestLevel/Blueprints/HUD_Tutorial.HUD_Tutorial_C"))
  (UserInterface|Viewport|AddtoViewport _returnvalue 0))

(fn HudOFF
  (bind _foundwidgets (Widget|GetAllWidgetsOfClass "/Game/Maps/Test/SushantTestLevel/Blueprints/HUD_Tutorial.HUD_Tutorial_C" true))
  (Widget|RemovefromParent (Utilities|Array|Get(acopy) _foundwidgets)))

(event Custom|3rd%20dialogue
  (Variables|Default|SetTutorialText (Variables|Default|GetTutorialText3))
  (Utilities|HudonOff))

(event Custom|1st%20dialogue
  (Variables|Default|SetTutorialText (Variables|Default|GetTutorialText1))
  (Utilities|HudonOff))

(event Custom|2nd%20dialogue
  (Variables|Default|SetTutorialText (Variables|Default|GetTutorialText2))
  (Utilities|HudonOff))

(event OnComponentBeginOverlap(Sphere)
  (params (OverlappedComponent :type Primitive%20Component%20Object%20Reference) (OtherActor :type Actor%20Object%20Reference) (OtherComp :type Primitive%20Component%20Object%20Reference) (OtherBodyIndex :type Integer) (bFromSweep :type Boolean) (SweepResult :type Hit%20Result%20Structure%20%28by%20ref%29))
  (bind _boxtriggers (Variables|Default|GetBoxTriggers))
  (Utilities|FlowControl|Sequence
    (:then_0
      (if (== OtherActor (Utilities|Array|Get(acopy) _boxtriggers))
        (CallFunction|1stDialogue)))
    (:then_1
      (if (== OtherActor (Utilities|Array|Get(acopy) _boxtriggers 1))
        (CallFunction|2ndDialogue)))
    (:then_2
      (if (== OtherActor (Utilities|Array|Get(acopy) _boxtriggers 2))
        (CallFunction|3rdDialogue)))))