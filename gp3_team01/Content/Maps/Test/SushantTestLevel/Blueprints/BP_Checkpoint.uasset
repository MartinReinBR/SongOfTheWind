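; BP_Checkpoint is a test-level checkpoint actor that updates the spawn transform held by the death zone when the player reaches it.
; On BeginPlay it caches the Bp_deathzone returned by GetActorOfClass, so only one death zone is updated.
; When player pawn 0 overlaps its Box, it writes its Arrow's world transform to that death zone's SpawnTransform and prints the value for debugging.
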(event OnComponentBeginOverlap(Box)
  (params (OverlappedComponent :type Primitive%20Component%20Object%20Reference) (OtherActor :type Actor%20Object%20Reference) (OtherComp :type Primitive%20Component%20Object%20Reference) (OtherBodyIndex :type Integer) (bFromSweep :type Boolean) (SweepResult :type Hit%20Result%20Structure%20%28by%20ref%29))
  (if (== OtherActor (Game|Player|GetPlayerPawn 0))
    (bind _output_get (Variables|/Game/Maps/Test/SushantTestLevel/Blueprints/bp_deathzone.bp_deathzone_C|SetSpawnTransform (stale EventBeginPlay _output_get) (Transformation|GetWorldTransform (Variables|Default|GetArrow))))
    (Development|PrintString (Utilities|String|ToString(Transform) _output_get))))

(event EventBeginPlay
  (bind _returnvalue (Actor|GetActorOfClass "/Game/Maps/Test/SushantTestLevel/Blueprints/bp_deathzone.bp_deathzone_C"))
  (bind _output_get (Variables|Default|SetDeathzone _returnvalue)))

(fn ConstructionScript)