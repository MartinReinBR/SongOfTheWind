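; Test-level death teleporter that hides the player, teleports to a Respawnpoint actor's transform, then reveals the player after a delay.
; Box overlap by the player character sends it the TeleportButton interface message, while this actor's TeleportButton event runs the sequence.
; StaticMeshOFF and StaticMeshON macros toggle player visibility with brief tutorial particle bursts.
; The mesh's visibility and collision are only switched off; input locking remains a noted TODO.
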(event OnComponentBeginOverlap(Box)
  (params (OverlappedComponent :type Primitive%20Component%20Object%20Reference) (OtherActor :type Actor%20Object%20Reference) (OtherComp :type Primitive%20Component%20Object%20Reference) (OtherBodyIndex :type Integer) (bFromSweep :type Boolean) (SweepResult :type Hit%20Result%20Structure%20%28by%20ref%29))
  ;[0 0 0] This actually checks if the player is inside the interactable collision
  (if (== OtherActor (stale EventBeginPlay _returnvalue))
    (Class|IntInteract|TeleportButton(Message) (stale EventBeginPlay _returnvalue))))

(event EventBeginPlay
  (bind _returnvalue (Actor|GetActorOfClass "/Game/Blueprints/Player/BP_FG_PlayerCharacter.BP_FG_PlayerCharacter_C")))

(event EventTeleportButton
  ;[1 0.9994 0 1 25] This is an interface event that will teleport the player
  (CallFunction|CallplayerChar)
  ;;[0 0 0] make sure to add a particle effect in here when ready
  (Utilities|StaticMeshOFF)
  (Utilities|Teleport)
  (Utilities|FlowControl|Delay 1.0)
  ;;[0 0 0] make sure to add a particle effect in here when ready
  (Utilities|StaticMeshON))

(fn ConstructionScript)

(fn CallplayerChar
  (bind _returnvalue (Actor|GetActorOfClass "/Game/Blueprints/Player/BP_FG_PlayerCharacter.BP_FG_PlayerCharacter_C"))
  (Variables|Default|Setplayerchar _returnvalue))