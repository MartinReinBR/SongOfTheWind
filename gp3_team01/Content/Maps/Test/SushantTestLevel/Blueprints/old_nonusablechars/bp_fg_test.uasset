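; Test player Blueprint with a pause menu, an interact key and respawn on death.
; Key 1 flip-flops macros that show or remove the pause HUD, noted in the graph as broken.
; A box overlap caches Int_interact actors so F can send them the teleport button message.
; When destroyed, it spawns a TargetPoint above itself, fades the camera from black and spawns a replacement at the Deathpedestal, without possessing it.
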(event Collision|EventActorBeginOverlap
  (params (OtherActor :type Actor%20Object%20Reference))
  (|CallParentFunction OtherActor) ; This node is disabled and will not be called.\nDrag off pins to build functionality.
)

(event Input|KeyboardEvents|1
  (params (Key :type Key%20Structure))
  ;[1 1 1] This is a pausemenu, replace the 1 button with whatever we will choose.
  (:Pressed
    (Utilities|FlowControl|FlipFlop
      (:A
        ;;[1 1 1] this turns the HUD on,
        (Utilities|HUDon (stale _returnvalue) (stale _returnvalue)))
      (:B
        ;;[1 1 1] this is not working, try to fix it sushant
        (bind _returnvalue (Utilities|DisablestheMenu))))))

(event Input|KeyboardEvents|F
  (params (Key :type Key%20Structure))
  ;[1 0 0.7313 1 25] This is an Interact Button (Keep adding more INTERACT functions after the teleport button)
  (:Pressed
    (Class|IntInteract|TeleportButton(Message) (Variables|Default|GetInterfaceActor))))

(event Custom|PlayerDestroyed
  (params (DestroyedActor :type Actor%20Object%20Reference))
  (bind _returnvalue (Transformation|GetActorTransform DestroyedActor))
  (Game|SpawnActorfromClass "/Script/Engine.TargetPoint" (Math|Transform|MakeTransform (Math|Vector|MakeVector (.x (.location _returnvalue)) (.y (.location _returnvalue)) (+ (.z (.location _returnvalue)) 1e+03)) (.rotation _returnvalue) "1,1,1") "AdjustIfPossibleButAlwaysSpawn" 0 0)
  (CameraFades|StartCameraFade (Game|GetPlayerCameraManager 0) 1.0 0.0 3.0 "(R=0.000000,G=0.000000,B=0.000000,A=1.000000)" true false)
  (bind _returnvalue_2 (Actor|GetActorOfClass "/Game/Maps/Test/SushantTestLevel/Blueprints/deathpedestal.deathpedestal_C"))
  (Game|SpawnActorfromClass "bp_fg_test_C" (Transformation|GetActorTransform _returnvalue_2) "Undefined" 0 0))

(event EventBeginPlay
  (Game|BindEventtoOnDestroyed (delegate Custom|PlayerDestroyed)))

(fn ConstructionScript
  (|CallParentFunction))

(event OnComponentBeginOverlap(Box)
  (params (OverlappedComponent :type Primitive%20Component%20Object%20Reference) (OtherActor :type Actor%20Object%20Reference) (OtherComp :type Primitive%20Component%20Object%20Reference) (OtherBodyIndex :type Integer) (bFromSweep :type Boolean) (SweepResult :type Hit%20Result%20Structure%20%28by%20ref%29))
  (if (Utilities|DoesObjectImplementInterface OtherActor "/Game/Maps/Test/SushantTestLevel/Interfaces/int_interact.int_interact_C")
    (Variables|Default|SetInterfaceActor OtherActor)))

(event OnComponentEndOverlap(Box)
  (params (OverlappedComponent :type Primitive%20Component%20Object%20Reference) (OtherActor :type Actor%20Object%20Reference) (OtherComp :type Primitive%20Component%20Object%20Reference) (OtherBodyIndex :type Integer))
  (if (== OtherActor (Variables|Default|GetInterfaceActor))
    (Variables|Default|SetInterfaceActor 0)))