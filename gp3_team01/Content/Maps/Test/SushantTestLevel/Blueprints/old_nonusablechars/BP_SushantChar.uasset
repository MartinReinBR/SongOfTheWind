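; BP_SushantChar is a test player character with respawning, a pause menu toggle and interaction.
; When destroyed, it spawns a new copy of itself at the Deathpedestal actor's transform.
; Caps Lock alternately loads and unloads the Pausemenu streaming level, leaving older widget-based pause logic unconnected.
; Its Collider tracks overlapping Int_interact actors, and F sends InteractButtonMessage to the stored one.
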(event Custom|PlayerDestroyed
  (params (DestroyedActor :type Actor%20Object%20Reference))
  (bind _returnvalue (Actor|GetActorOfClass "/Game/Maps/Test/SushantTestLevel/Blueprints/deathpedestal.deathpedestal_C"))
  (Game|SpawnActorfromClass "BP_SushantChar_C" (Transformation|GetActorTransform _returnvalue) "Undefined" 0 0))

(event EventBeginPlay
  (|CallParentFunction)
  (Game|BindEventtoOnDestroyed (delegate Custom|PlayerDestroyed)))

(event Collision|EventActorBeginOverlap
  (params (OtherActor :type Actor%20Object%20Reference))
  (|CallParentFunction OtherActor) ; This node is disabled and will not be called.\nDrag off pins to build functionality.
)

(event Input|KeyboardEvents|CapsLock
  (params (Key :type Key%20Structure :default "None"))
  (:Pressed
    (Utilities|FlowControl|FlipFlop
      (:A
        (Class|GameplayStatics|LoadStreamLevelbySoftObjectPtr "/Game/Maps/Test/SushantTestLevel/Maps/pausemenu.pausemenu" true false))
      (:B
        (Game|UnloadStreamLevel(byName) "pausemenu" false)))))

(fn ConstructionScript
  (|CallParentFunction))

(event OnComponentBeginOverlap(Collider)
  (params (OverlappedComponent :type Primitive%20Component%20Object%20Reference) (OtherActor :type Actor%20Object%20Reference) (OtherComp :type Primitive%20Component%20Object%20Reference) (OtherBodyIndex :type Integer) (bFromSweep :type Boolean) (SweepResult :type Hit%20Result%20Structure%20%28by%20ref%29))
  (if (Utilities|DoesObjectImplementInterface OtherActor "/Game/Maps/Test/SushantTestLevel/Interfaces/int_interact.int_interact_C")
    (Variables|Default|SetInteractActor OtherActor)))

(event OnComponentEndOverlap(Collider)
  (params (OverlappedComponent :type Primitive%20Component%20Object%20Reference) (OtherActor :type Actor%20Object%20Reference) (OtherComp :type Primitive%20Component%20Object%20Reference) (OtherBodyIndex :type Integer))
  (if (== OtherActor (Variables|Default|GetInteractActor))
    (Variables|Default|SetInteractActor 0)))

(event Input|KeyboardEvents|F
  (params (Key :type Key%20Structure :default "None"))
  (:Pressed
    (Class|IntInteract|InteractButton(Message) (Variables|Default|GetinteractActor))))