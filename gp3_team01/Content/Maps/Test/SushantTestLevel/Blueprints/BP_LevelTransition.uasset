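; BP_LevelTransition is a trigger volume that moves the player to another level when their pawn overlaps its box.
; On overlap it fades the camera and audio, adds a HUD_LoadingScreen widget, fades again, then opens the level held in its Level variable.
; Fixed delays sequence the steps, and the loading widget is removed right after the open-level call.
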(event OnComponentBeginOverlap(Box)
  (params (OverlappedComponent :type Primitive%20Component%20Object%20Reference) (OtherActor :type Actor%20Object%20Reference) (OtherComp :type Primitive%20Component%20Object%20Reference) (OtherBodyIndex :type Integer) (bFromSweep :type Boolean) (SweepResult :type Hit%20Result%20Structure%20%28by%20ref%29))
  (if (== OtherActor (Game|Player|GetPlayerPawn 0))
    (CameraFades|StartCameraFade :self (Game|GetPlayerCameraManager 0) :ToAlpha 2.0 :Duration 2.0 :bShouldFadeAudio true :bHoldWhenFinished true)
    (Utilities|FlowControl|Delay 2.0)
    (bind _returnvalue (UserInterface|CreateWidget "/Game/Blueprints/Menu/HUD_LoadingScreen.HUD_LoadingScreen_C"))
    (UserInterface|Viewport|AddtoViewport _returnvalue 0)
    (Utilities|FlowControl|Delay 2.0)
    (CameraFades|StartCameraFade (Game|GetPlayerCameraManager 0) 0.0 1.0 2.0 "(R=0.000000,G=0.000000,B=0.000000,A=1.000000)" true true)
    (Utilities|FlowControl|Delay 2.0)
    (Game|OpenLevel(byObjectReference) (Variables|Default|GetLevel))
    (Widget|RemovefromParent _returnvalue)))

(fn ConstructionScript)