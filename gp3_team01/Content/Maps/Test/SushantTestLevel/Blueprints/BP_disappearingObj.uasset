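; BP_disappearingObj is a test-level object that temporarily vanishes after something lands on it.
; The locomotion land event waits briefly, hides the cube and disables its collision, then restores both after a second delay.
; The MeshOff and MeshOn functions handle the visibility and collision toggles.
; Leftover nodes for teleporting to a Deathpedestal actor are unconnected and never run.
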(event EventOnLocomotionLand
  (params (LocomotionComponentOfCaller :type FG%20Locomotion%20Component%20Object%20Reference))
  (Utilities|FlowControl|Delay 1.0)
  (Utilities|MeshOff)
  (Utilities|FlowControl|Delay 1.0)
  (Utilities|Meshon))

(fn ConstructionScript)