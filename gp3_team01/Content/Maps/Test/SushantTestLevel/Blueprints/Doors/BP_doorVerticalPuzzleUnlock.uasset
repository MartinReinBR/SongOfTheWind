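; Test-level vertical puzzle door Blueprint, apparently unfinished, with events to unlock and lock the door.
; UnlockDoorVertical hides the door mesh either way, disabling collision only if the puzzle element read from Tick's otherwise empty loop is unlocked.
; LockDoorVertical reverses a timeline that lerps the door's Z position, but sets play rate on a different timeline.
; The animated opening and the search for puzzle actors are unconnected.
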(event EventBeginPlay)

(event EventUnlockDoorVertical
  (bind _actualdoor (Variables|Default|GetActualDoor))
  (bind _actualdoor_2 (Variables|Default|GetActualDoor))
  (if (Variables|/Game/Maps/Test/SushantTestLevel/Blueprints/PuzzleUnlockers/bp_unlockdoorVertical.bp_unlockdoorVertical_C|GetPuzzleUnlocked (stale EventTick _array_element))
    (Rendering|SetVisibility _actualdoor false false)
    (Collision|SetCollisionEnabled _actualdoor "NoCollision")
    (else
      (Rendering|SetVisibility _actualdoor_2 false false)
      (Collision|SetCollisionEnabled _actualdoor_2 "QueryAndPhysics"))))

(event EventLockDoorVertical
  ;[1 1 1] DoorFunctionality Close
  (Components|Timeline|SetPlayRate (Variables|Default|GetDoorAnimationLeft) 2.0)
  (bind _leftdooropen (Timeline|Timeline_0 Reverse)
    (:Update
      (Transformation|SetRelativeLocation (Variables|Default|GetActualDoor) (Math|Vector|MakeVector 0.0 0.0 (Math|Float|Lerp (Variables|Default|GetLeftDoorCloseFloat) (Variables|Default|GetLeftDoorOpenFloat) _leftdooropen)) false false))))

(event EventTick
  (params (DeltaSeconds :type Float%20%28single-precision%29))
  (for _array_element (Variables|Default|GetPuzzlearray)
    _))

(fn ConstructionScript)