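; Double sliding door in a test level that opens when the first player's pawn enters its box trigger and closes when it leaves.
; Entering plays one timeline per panel at double rate, lerping each panel's relative X between closed and open values.
; Leaving runs a separate pair of timelines in reverse from the end, while the play-rate calls still target the opening timelines.
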(event OnComponentBeginOverlap(Box)
  (params (OverlappedComponent :type Primitive%20Component%20Object%20Reference) (OtherActor :type Actor%20Object%20Reference) (OtherComp :type Primitive%20Component%20Object%20Reference) (OtherBodyIndex :type Integer) (bFromSweep :type Boolean) (SweepResult :type Hit%20Result%20Structure%20%28by%20ref%29))
  (if (== OtherActor (Game|Player|GetPlayerPawn 0))
    ;[1 1 1] DoorFunctionality Open
    (Utilities|FlowControl|Sequence
      (:then_0
        (Components|Timeline|SetPlayRate (Variables|Default|GetDoorAnimationLeft) 2.0)
        (bind _leftdooropen (Timeline|DoorAnimationLeft Play)
          (:Update
            (Transformation|SetRelativeLocation (Variables|Default|GetActualDoorLeft) (Math|Vector|MakeVector (Math|Float|Lerp (Variables|Default|GetLeftDoorCloseFloat) (Variables|Default|GetLeftDoorOpenFloat) _leftdooropen) 0.0 0.0) false false))))
      (:then_1
        (Components|Timeline|SetPlayRate (Variables|Default|GetDoorAnimationRight) 2.0)
        (bind _rightdooropen (Timeline|DoorAnimationRight Play)
          (:Update
            (Transformation|SetRelativeLocation (Variables|Default|GetActualDoorRight) (Math|Vector|MakeVector (Math|Float|Lerp (Variables|Default|GetRightDoorCloseFloat) (Variables|Default|GetRightDoorOpenFloat) _rightdooropen) 0.0 0.0) false false)))))))

(event OnComponentEndOverlap(Box)
  (params (OverlappedComponent :type Primitive%20Component%20Object%20Reference) (OtherActor :type Actor%20Object%20Reference) (OtherComp :type Primitive%20Component%20Object%20Reference) (OtherBodyIndex :type Integer))
  (if (== OtherActor (Game|Player|GetPlayerPawn 0))
    ;[1 1 1] DoorFunctionality Close
    (Utilities|FlowControl|Sequence
      (:then_0
        (Components|Timeline|SetPlayRate (Variables|Default|GetDoorAnimationLeft) 2.0)
        (bind _leftdooropen (Timeline|Timeline_0 ReverseFromEnd)
          (:Update
            (Transformation|SetRelativeLocation (Variables|Default|GetActualDoorLeft) (Math|Vector|MakeVector (Math|Float|Lerp (Variables|Default|GetLeftDoorCloseFloat) (Variables|Default|GetLeftDoorOpenFloat) _leftdooropen) 0.0 0.0) false false))))
      (:then_1
        (Components|Timeline|SetPlayRate (Variables|Default|GetDoorAnimationRight) 2.0)
        (bind _rightdooropen (Timeline|Timeline_1 ReverseFromEnd)
          (:Update
            (Transformation|SetRelativeLocation (Variables|Default|GetActualDoorRight) (Math|Vector|MakeVector (Math|Float|Lerp (Variables|Default|GetRightDoorCloseFloat) (Variables|Default|GetRightDoorOpenFloat) _rightdooropen) 0.0 0.0) false false)))))))

(fn ConstructionScript)