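; Test-level sliding double door that opens sideways when a puzzle (Bp_unlockdoor) reports it is unlocked.
; BeginPlay gathers all puzzle actors, and Tick loops over them with an empty body.
; UnlockDoorSideways checks the loop element's PuzzleUnlocked flag, turns Pillar2 green or red, and opens or closes both panels through timeline-driven X-position lerps.
; LockDoorSideways jumps straight to the closing sequence, skipping the color change.
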(event EventBeginPlay
  (bind _outactors (Actor|GetAllActorsOfClass "/Game/Maps/Test/SushantTestLevel/Blueprints/PuzzleUnlockers/bp_unlockdoor.bp_unlockdoor_C"))
  (bind _output_get (Variables|Default|SetPuzzlesToBeUnlocked _outactors)))

(event EventUnlockDoorSideways
  (bind _pillar2 (Variables|Default|GetPillar2))
  (if (Variables|/Game/Maps/Test/SushantTestLevel/Blueprints/PuzzleUnlockers/bp_unlockdoor.bp_unlockdoor_C|GetPuzzleUnlocked (stale EventTick _array_element))
    (Rendering|Material|SetMaterial _pillar2 0 "/Game/Maps/Test/SushantTestLevel/Assets/mat_debug_green.mat_debug_green")
    ;[1 1 1] DoorFunctionality Open
    (Utilities|FlowControl|Sequence
      (:then_0
        (Components|Timeline|SetPlayRate (Variables|Default|GetDoorAnimationLeft) 2.0)
        (bind _leftdooropen (Timeline|DoorAnimationLeft Play)
          (:Update
            (Transformation|SetRelativeLocation (Variables|Default|GetActualDoorLeft) (Math|Vector|MakeVector (Math|Float|Lerp (Variables|Default|GetLeftDoorCloseFloat) (Variables|Default|GetLeftDoorOpenFloat) _leftdooropen) 0.0 0.0) false false))))
      (:then_1
        (Components|Timeline|SetPlayRate (Variables|Default|GetDoorAnimationRight) 2.0)
        (bind _rightdooropen (Timeline|DoorAnimationRight Play)
          (:Update
            (Transformation|SetRelativeLocation (Variables|Default|GetActualDoorRight) (Math|Vector|MakeVector (Math|Float|Lerp (Variables|Default|GetRightDoorCloseFloat) (Variables|Default|GetRightDoorOpenFloat) _rightdooropen) 0.0 0.0) false false)))))
    (else
      (Rendering|Material|SetMaterial _pillar2 0 "/Game/Maps/Test/SushantTestLevel/Assets/mat_debug_red.mat_debug_red")
      ;[1 1 1] DoorFunctionality Close
      (Utilities|FlowControl|Sequence
        (:then_0
          (Components|Timeline|SetPlayRate (Variables|Default|GetDoorAnimationLeft) 2.0)
          (bind _leftdooropen_2 (Timeline|Timeline_0 Reverse)
            (:Update
              (Transformation|SetRelativeLocation (Variables|Default|GetActualDoorLeft) (Math|Vector|MakeVector (Math|Float|Lerp (Variables|Default|GetLeftDoorCloseFloat) (Variables|Default|GetLeftDoorOpenFloat) _leftdooropen_2) 0.0 0.0) false false))))
        (:then_1
          (Components|Timeline|SetPlayRate (Variables|Default|GetDoorAnimationRight) 2.0)
          (bind _rightdooropen_2 (Timeline|Timeline_1 Reverse)
            (:Update
              (Transformation|SetRelativeLocation (Variables|Default|GetActualDoorRight) (Math|Vector|MakeVector (Math|Float|Lerp (Variables|Default|GetRightDoorCloseFloat) (Variables|Default|GetRightDoorOpenFloat) _rightdooropen_2) 0.0 0.0) false false))))))))

(event EventLockDoorSideways
  ;[1 1 1] DoorFunctionality Close
  (Utilities|FlowControl|Sequence
    (:then_0
      (Components|Timeline|SetPlayRate (Variables|Default|GetDoorAnimationLeft) 2.0)
      (bind _leftdooropen (Timeline|Timeline_0 Reverse)
        (:Update
          (Transformation|SetRelativeLocation (Variables|Default|GetActualDoorLeft) (Math|Vector|MakeVector (Math|Float|Lerp (Variables|Default|GetLeftDoorCloseFloat) (Variables|Default|GetLeftDoorOpenFloat) _leftdooropen) 0.0 0.0) false false))))
    (:then_1
      (Components|Timeline|SetPlayRate (Variables|Default|GetDoorAnimationRight) 2.0)
      (bind _rightdooropen (Timeline|Timeline_1 Reverse)
        (:Update
          (Transformation|SetRelativeLocation (Variables|Default|GetActualDoorRight) (Math|Vector|MakeVector (Math|Float|Lerp (Variables|Default|GetRightDoorCloseFloat) (Variables|Default|GetRightDoorOpenFloat) _rightdooropen) 0.0 0.0) false false))))))

(event EventTick
  (params (DeltaSeconds :type Float%20%28single-precision%29))
  (for _array_element (stale EventBeginPlay _output_get)
    _))

(fn ConstructionScript)