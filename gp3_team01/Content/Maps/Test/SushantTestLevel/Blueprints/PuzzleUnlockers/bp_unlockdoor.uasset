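; Rotatable puzzle piece that unlocks a sideways puzzle door when its line trace hits an actor tagged "unlocker".
; Box overlap sends the player pawn an interact-button message, and the InteractButton event rotates Sphere 90 degrees.
; Every tick, a multi-trace from Arrow to Sphere1 calls Unlocked or Locked per hit, or Locked without one.
; Both message the first BP_doorSidewaysPuzzleUnlock found at BeginPlay.
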(event OnComponentBeginOverlap(Box)
  (params (OverlappedComponent :type Primitive%20Component%20Object%20Reference) (OtherActor :type Actor%20Object%20Reference) (OtherComp :type Primitive%20Component%20Object%20Reference) (OtherBodyIndex :type Integer) (bFromSweep :type Boolean) (SweepResult :type Hit%20Result%20Structure%20%28by%20ref%29))
  (bind _returnvalue (Game|Player|GetPlayerPawn 0))
  (bind _returnvalue_2 (== OtherActor _returnvalue))
  (if _returnvalue_2
    (if _returnvalue_2
      (Class|IntInteract|InteractButton(Message) _returnvalue)
      (Development|PrintString "Hello"))))

(event EventBeginPlay
  (bind _outactors (Actor|GetAllActorsOfClass "/Game/Maps/Test/SushantTestLevel/Blueprints/Doors/BP_doorSidewaysPuzzleUnlock.BP_doorSidewaysPuzzleUnlock_C"))
  (Variables|Default|SetHorizontalPuzzleActor _outactors))

(event EventInteractButton
  (Transformation|AddRelativeRotation (Variables|Default|GetSphere) "0,90.000000, 0" false false))

(event EventTick
  (params (DeltaSeconds :type Float%20%28single-precision%29))
  (bind (_outhits _returnvalue) (Collision|MultiLineTraceByChannel (Transformation|GetWorldLocation (Variables|Default|GetArrow)) (Transformation|GetWorldLocation (Variables|Default|GetSphere1)) "TraceTypeQuery1" true (Utilities|Array|MakeArray (Game|Player|GetPlayerPawn 0)) "ForOneFrame" true "(R=1.000000,G=0.000000,B=0.000000,A=1.000000)" "(R=0.000000,G=1.000000,B=0.000000,A=1.000000)" 2.0))
  (if _returnvalue
    (bind _array_element (Utilities|Array|ForEachLoopwithBreak _outhits)
      (:LoopBody
        (if (Actor|ActorHasTag (.HitActor (Collision|BreakHitResult _array_element)) "unlocker")
          (CallFunction|Unlocked)
          (else
            (CallFunction|Locked)))))
    (else
      (CallFunction|Locked))))

(fn ConstructionScript)

(fn Unlocked
  (Variables|Default|SetPuzzleUnlocked true)
  (Class|IntUnlockdoor|UnlockDoorSideways(Message) (Utilities|Array|Get(acopy) (Variables|Default|GetHorizontalPuzzleActor))))

(fn Locked
  (Variables|Default|SetPuzzleUnlocked false)
  (Class|IntUnlockdoor|LockDoorSideways(Message) (Utilities|Array|Get(acopy) (Variables|Default|GetHorizontalPuzzleActor))))