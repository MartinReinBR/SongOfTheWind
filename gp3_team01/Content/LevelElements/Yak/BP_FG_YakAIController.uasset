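; AI controller for the Yak level element that drives its behavior through a blackboard and behavior tree.
; On possess it initializes the yak blackboard, runs the yak behavior tree and prints a leftover debug string.
; On any target perception update, if the Player key holds no valid object, it stores the first player character found in the world, ignoring what was actually sensed.
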(event OnTargetPerceptionUpdated(PerceptionComponent)
  (params (Actor :type Actor%20Object%20Reference) (Stimulus :type AI%20Stimulus%20Structure))
  (if (not (Utilities|IsValid (AI|Components|Blackboard|GetValueasObject (Variables|Default|GetBlackboard%20Component) (Variables|Default|GetPlayer))))
    (bind _outactors (Actor|GetAllActorsOfClass "/Game/Blueprints/Player/BP_FG_PlayerCharacter.BP_FG_PlayerCharacter_C"))
    (AI|Components|Blackboard|SetValueasObject (Variables|Default|GetBlackboard%20Component) (Variables|Default|GetPlayer) (Utilities|Array|Get(acopy) _outactors))))

(event EventBeginPlay)

(event EventTick
  (params (DeltaSeconds :type Float%20%28single-precision%29)))

(event EventPossess
  (params (PossessedPawn :type Pawn%20Object%20Reference))
  (bind _blackboardcomponent (Class|AIController|UseBlackboard "/Game/LevelElements/Yak/BB_FG_YakAICharacter.BB_FG_YakAICharacter"))
  (Variables|Default|SetBlackboard%20Component _blackboardcomponent)
  (AI|RunBehaviorTree "/Game/LevelElements/Yak/BT_FG_YakAICharacter.BT_FG_YakAICharacter")
  (Development|PrintString "DAB"))

(fn ConstructionScript)