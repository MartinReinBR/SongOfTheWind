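; BP_FG_Winddraft is a wind draft level element that drives a Niagara wind effect.
; On BeginPlay it sets the speck, ribbon and windpuff spawn rates, each from its own multiplier scaled by a shared particle multiplier.
; Unconnected leftover logic would call ApplyWindForce on the player character and print a debug string, but it never runs, so this graph only configures visuals.
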(event EventBeginPlay
  (bind _niagara (Variables|Default|GetNiagara))
  (bind _particlemultiplier (Variables|Default|GetParticleMultiplier))
  (Niagara|SetNiagaraVariable(Float) _niagara "SpeckSpawnrate" (* (Variables|Default|GetSpeckMultiplier) _particlemultiplier))
  (Niagara|SetNiagaraVariable(Float) _niagara "RibbonSpawnrate" (* (Variables|Default|GetRibbonMultiplier) _particlemultiplier))
  (Niagara|SetNiagaraVariable(Float) _niagara "WindpuffSpawnrate" (* (Variables|Default|GetPuffMultiplier) _particlemultiplier)))

(event Collision|EventActorBeginOverlap
  (params (OtherActor :type Actor%20Object%20Reference)))

(event EventTick
  (params (DeltaSeconds :type Float%20%28single-precision%29)))

(fn ConstructionScript)