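; Lotus collectible Blueprint that responds to being collected by a player character.
; On collect it scales its owner to half size, hides itself and adds itself to the character's Collector.
; It then increments Score by one and prints the new total on screen in gold text.
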(event EventBeginPlay)

(event EventTick
  (params (DeltaSeconds :type Float%20%28single-precision%29)))

(event EventOnCollect
  (params (PlayerCharacter :type FG%20Player%20Character%20Object%20Reference))
  (bind _score (Variables|Default|GetScore))
  (Transformation|SetActorScale3D (Components|GetOwner) "0.500000,0.500000,0.500000")
  (Class|FGCollectibleComponent|HideSelf true)
  (Class|FGCollectorComponent|Add (Variables|/Script/gp3_team01.FG_PlayerCharacter|GetCollector PlayerCharacter) self)
  (Class|DAFGIntegerData|Increment _score 1)
  (Development|PrintString (Utilities|String|ToString(Integer) (Class|DAFGIntegerData|Get _score)) true true "(R=1.000000,G=0.750000,B=0.000000,A=1.000000)"))