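; Jump lotus collectible that bounces the collecting player upward and grants another double jump.
; On collect it hides, pushes the airborne sub-state, clears vertical velocity while keeping horizontal motion, then applies a raw jump through the locomotion component.
; A countdown in Tick shows the lotus again after a short delay, making it reusable.
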(event EventBeginPlay)

(event EventTick
  (params (DeltaSeconds :type Float%20%28single-precision%29))
  (if (>= (Variables|Default|GetTimer) -0.01)
    (bind _output_get (Variables|Default|SetTimer (- (Variables|Default|GetTimer) DeltaSeconds)))
    (if (< _output_get 0.0)
      (Class|FGCollectibleComponent|ShowSelf))))

(event EventOnCollect
  (params (PlayerCharacter :type FG%20Player%20Character%20Object%20Reference))
  (bind _collider (Variables|/Script/gp3_team01.FG_PlayerCharacter|GetCollider PlayerCharacter))
  (bind _locomotioncorestate (Variables|/Script/gp3_team01.FG_PlayerCharacter|GetLocomotionCoreState PlayerCharacter))
  (Class|FGCollectibleComponent|HideSelf false)
  (Class|FGSFSM|Push (Variables|/Script/gp3_team01.FG_LocomotionPlayerState|GetSubStateMachine _locomotioncorestate) (Variables|/Script/gp3_team01.FG_LocomotionPlayerState|GetLocomotionAirborneSubState _locomotioncorestate))
  (bind _returnvalue (Physics|GetPhysicsLinearVelocity _collider "None"))
  (Physics|SetPhysicsLinearVelocity _collider (Math|Vector|MakeVector (.x _returnvalue) (.y _returnvalue) 0.0) false "None")
  (Class|FGLocomotionComponent|JumpRAW (Variables|/Script/gp3_team01.FG_PlayerCharacter|GetLocomotionComp PlayerCharacter) 1e+03 0.0 0.0)
  (Variables|Default|SetTimer 2.0)
  (Class|FGPlayerCharacter|AllowAnotherDoubleJump PlayerCharacter))