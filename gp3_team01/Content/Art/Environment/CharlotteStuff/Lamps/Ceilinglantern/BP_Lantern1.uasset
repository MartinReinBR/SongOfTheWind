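; BP_Lantern1 is a ceiling lantern prop that changes state when the player pawn walks into its Box trigger.
; BeginPlay toggles the visibility of UrnSeparate, and a player overlap sets it visible, destroys the existing Niagara effect, adds a new one and plays a sound at world origin.
; InteractButton is an empty event, and nothing guards against repeated overlaps.
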(event OnComponentBeginOverlap(Box)
  (params (OverlappedComponent :type Primitive%20Component%20Object%20Reference) (OtherActor :type Actor%20Object%20Reference) (OtherComp :type Primitive%20Component%20Object%20Reference) (OtherBodyIndex :type Integer) (bFromSweep :type Boolean) (SweepResult :type Hit%20Result%20Structure%20%28by%20ref%29))
  (if (== (Game|Player|GetPlayerPawn 0) OtherActor)
    (AddComponent|AddNiagaraComponent false (Variables|Default|GetNewVar_0))
    (Components|DestroyComponent (Variables|Default|GetNiagara))
    (Rendering|ToggleVisibility (Variables|Default|Geturn_separate) true)
    (Audio|PlaySoundatLocation "/Game/Audio/Sounds/CloudDrum_Default/CD_Default_A5.CD_Default_A5" "0, 0, 0" "0, 0, 0" 1.0 1.0 0.0 0 0 0)))

(event EventInteractButton)

(event EventBeginPlay
  (Rendering|ToggleVisibility (Variables|Default|Geturn_separate) false))

(fn ConstructionScript)